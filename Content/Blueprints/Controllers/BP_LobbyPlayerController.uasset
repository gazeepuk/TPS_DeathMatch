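; Player controller for the multiplayer lobby that owns the local player's lobby menu and in-game menu widgets.
; On BeginPlay, the local controller adds the default input mapping context, creates the lobby menu, refreshes its player list and enables Game and UI input with a cursor.
; UpdatePlayerList forwards refreshes to the lobby widget, creating it if missing.
; The game menu input shows the cached menu widget, creating it on first use.
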(event `self.ReceiveBeginPlay`
  (if (`self.IsLocalPlayerController`)
    (`EnhancedInputSubsystemInterface.AddMappingContext` (pcsubsystem `EnhancedInputLocalPlayerSubsystem` self) "/Game/Blueprints/Input/IMC_Default.IMC_Default" 0 (struct))
    (`self.SetupLobbyWidget`)))

(event `self.UpdatePlayerList`
  (if (`self.IsLocalPlayerController`)
    (`/Engine/EditorBlueprintResources/StandardMacros.IsValid` (`self.LobbyMenu`)
      (:`Is Valid`
        _)
      (:`Is Not Valid`
        (`self.CreateLobbyMenuWidget`)
        (`/Engine/EditorBlueprintResources/StandardMacros.IsValid` (`self.LobbyMenu`)
          (:`Is Valid`
            _))))
    (`/Game/Blueprints/UI/Lobby/WBP_LobbyMenu.UpdatePlayerList` (`self.LobbyMenu`))))

(event `EnhancedInput|/Game/Blueprints/Input/Actions/IA_GameMenu`
  (params (ActionValue :type Boolean) (ElapsedSeconds :type "Float (double-precision)") (TriggeredSeconds :type "Float (double-precision)") (InputAction :type "InputAction Object Reference" :default "/Game/Blueprints/Input/Actions/IA_GameMenu.IA_GameMenu"))
  (bind _gamemenuwidget (`self.GameMenuWidget`))
  (:`Started`
    (`/Engine/EditorBlueprintResources/StandardMacros.IsValid` (`self.GameMenuWidget`)
      (:`Is Valid`
        (`Widget.SetVisibility` _gamemenuwidget "Visible")
        (`UserWidget.AddToViewport` _gamemenuwidget 0))
      (:`Is Not Valid`
        (bind _returnvalue (`|CreateWidget` "/Game/Blueprints/UI/MainMenu/WBP_GameMenu.WBP_GameMenu_C" self))
        (bind _output_get (set `self.GameMenuWidget` _returnvalue))
        (`UserWidget.AddToViewport` _output_get 0)))
    (`WidgetBlueprintLibrary.SetInputMode_GameAndUIEx` self null)
    (set `self.bShowMouseCursor` true)))

(fn `CreateLobbyMenuWidget`
  (bind _returnvalue (`|CreateWidget` "/Game/Blueprints/UI/Lobby/WBP_LobbyMenu.WBP_LobbyMenu_C" self))
  (bind _output_get (set `self.LobbyMenu` _returnvalue))
  (`UserWidget.AddToViewport` _output_get 0))

(fn `SetupLobbyWidget`
  (if (`self.IsLocalPlayerController`)
    (`self.CreateLobbyMenuWidget`)
    (`self.UpdatePlayerList`)
    (`WidgetBlueprintLibrary.SetInputMode_GameAndUIEx` self null)
    (set `self.bShowMouseCursor` true)))

(fn `UserConstructionScript`)
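; Player controller for death match, judging by its name, that opens the in-game menu.
; When the game menu input action starts, it creates and caches a WBP_GameMenu widget, passing it a previous input mode, or makes the existing one visible.
; It then adds the menu to the viewport, switches input to Game and UI, and shows the mouse cursor.
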(event `EnhancedInput|/Game/Blueprints/Input/Actions/IA_GameMenu`
  (params (ActionValue :type Boolean) (ElapsedSeconds :type "Float (double-precision)") (TriggeredSeconds :type "Float (double-precision)") (InputAction :type "InputAction Object Reference" :default "/Game/Blueprints/Input/Actions/IA_GameMenu.IA_GameMenu"))
  (bind _gamemenuwidget (`self.GameMenuWidget`))
  (:`Started`
    (`/Engine/EditorBlueprintResources/StandardMacros.IsValid` (`self.GameMenuWidget`)
      (:`Is Valid`
        (`Widget.SetVisibility` _gamemenuwidget "Visible")
        (`UserWidget.AddToViewport` _gamemenuwidget 0))
      (:`Is Not Valid`
        (bind _returnvalue (`|CreateWidget` "/Game/Blueprints/UI/MainMenu/WBP_GameMenu.WBP_GameMenu_C" self "NewEnumerator1"))
        (bind _output_get (set `self.GameMenuWidget` _returnvalue))
        (`UserWidget.AddToViewport` _output_get 0)))
    (`WidgetBlueprintLibrary.SetInputMode_GameAndUIEx` self null)
    (set `self.bShowMouseCursor` true)))

(fn `UserConstructionScript`)